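; BP_UnitTest is a functional test that checks player pawn movement and robot spawning.
; On start it finds or spawns the PlayerPawn, calls its SpawnAnotherRobotActor, then records the pawn's location and all RobotActors.
; Each tick it pushes the pawn along negative world X, succeeding once it is over 500 units from the start and at least one robot was found.
; The graph has no explicit failure path.
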(event `self.ReceiveStartTest`
  (bind _playerpawn (`self.PlayerPawn`))
  ; Make the Correct pawn if it doesn't exist
  (`/Engine/EditorBlueprintResources/StandardMacros.IsValid` (`self.PlayerPawn`)
    (:`Is Valid`
      _)
    (:`Is Not Valid`
      (bind _returnvalue (`GameplayStatics.GetActorOfClass` "/Game/Actors/Player/PlayerPawn.PlayerPawn_C"))
      (`/Engine/EditorBlueprintResources/StandardMacros.IsValid` _returnvalue
        (:`Is Valid`
          (set `self.PlayerPawn` _returnvalue))
        (:`Is Not Valid`
          (bind _returnvalue_2 (`|SpawnActorFromClass` "/Game/Actors/Player/PlayerPawn.PlayerPawn_C" (`KismetMathLibrary.MakeTransform` (0.0 0.0 0.0)) "Undefined" "MultiplyWithRoot" null null))
          (set `self.PlayerPawn` _returnvalue_2)))))
  ; Tracking initial location and Check robot spawn functionality
  (`/Game/Actors/Player/PlayerPawn.Spawn another Robot Actor` _playerpawn)
  (set `self.Initial Position` (`self.K2_GetActorLocation` _playerpawn))
  (bind _outactors (`GameplayStatics.GetAllActorsOfClass` "/Game/Actors/RobotActor.RobotActor_C"))
  (set `self.Robot Actor List` _outactors))

(event `self.ReceiveTick`
  (params (DeltaSeconds :type "Float (single-precision)"))
  (bind _playerpawn (`self.PlayerPawn`))
  ; Moving backwards to check movement functionality
  (`Pawn.AddMovementInput` _playerpawn (-1.0 0.0 0.0) 1.0 false)
  (if (and (> (`KismetMathLibrary.Vector_Distance` (`self.K2_GetActorLocation` _playerpawn) (`self.Initial Position`)) 500.0) (> (`KismetArrayLibrary.Array_Length` (`self.Robot Actor List`)) 0))
    (`self.FinishTest` "Succeeded")))

(fn `UserConstructionScript`)